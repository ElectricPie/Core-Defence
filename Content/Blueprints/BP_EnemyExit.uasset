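; BP_EnemyExit is the tower defence exit point where enemies carrying a health orb cost the player health.
; It caches the first player controller as a BP_TowerDefencePlayer on BeginPlay.
; When a BasicEnemy overlaps its ExitTrigger and its HealthOrbSocket component holds an orb, it calls ReduceHealth on that controller and destroys the enemy.
; Enemies without an orb pass through unaffected.
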(event `self.ReceiveBeginPlay`
  (bind _asbp_tower_defence_player (cast `/Game/Blueprints/BP_TowerDefencePlayer` (`GameplayStatics.GetPlayerController` 0)))
  (set `self.PlayerController` _asbp_tower_defence_player))

(event `self.ExitTrigger.OnComponentBeginOverlap`
  (params (OverlappedComponent :type "PrimitiveComponent Object Reference") (OtherActor :type "Actor Object Reference") (OtherComp :type "PrimitiveComponent Object Reference") (OtherBodyIndex :type Integer) (bFromSweep :type Boolean) (SweepResult :type "HitResult Structure (by ref)"))
  (if (`KismetSystemLibrary.IsValid` (`self.PlayerController`))
    (bind _asbasic_enemy (cast `BasicEnemy` OtherActor))
    (if (`HealthOrbSocket.HasOrb` (`self.GetComponentByClass` _asbasic_enemy "/Script/GridTD.HealthOrbSocket"))
      (`TowerDefencePlayer.ReduceHealth` (`self.PlayerController`))
      (`self.K2_DestroyActor` _asbasic_enemy))))

(fn `UserConstructionScript`)