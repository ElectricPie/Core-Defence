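; BP_ChainTurret_1 is a chain turret Blueprint that handles the turret's visual response to aiming and firing events.
; Rotation and pitch updates are written into the ABP_ChainTurret_1 animation instance on TurretBaseMesh, which receives them as TurretRotation and TurretPitch.
; The fire event activates the FXExplosionBarrel effect with a reset, and the file contains no targeting or damage logic.
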(event `self.UpdateTurretRotation`
  (params (Rotation :type "Float (single-precision)"))
  (bind _asabp_chain_turret_1 (cast `/Game/Animations/ABP_ChainTurret_1` (`SkeletalMeshComponent.GetAnimInstance` (`self.TurretBaseMesh`))))
  (set `/Game/Animations/ABP_ChainTurret_1.TurretRotation` Rotation _asabp_chain_turret_1))

(event `self.UpdateTurretPitch`
  (params (Pitch :type "Float (single-precision)"))
  (bind _asabp_chain_turret_1 (cast `/Game/Animations/ABP_ChainTurret_1` (`SkeletalMeshComponent.GetAnimInstance` (`self.TurretBaseMesh`))))
  (set `/Game/Animations/ABP_ChainTurret_1.TurretPitch` Pitch _asabp_chain_turret_1))

(event `self.OnFireEvent`
  (`ActorComponent.Activate` (`self.FX_Explosion_Barrel`) true))

(fn `UserConstructionScript`)